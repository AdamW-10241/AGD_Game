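; BP_Pickup_Health is a health pickup that heals the player character on overlap and is then consumed.
; A box overlap casts to BP_AGDPlayerCharacter and continues only if its StatsComponent health is below maximum.
; The new health is a flat bonus added to current health, then multiplied, clamped to max and rounded up.
; It then plays a sound, spawns a heal particle effect and destroys itself, so full-health players leave it in place.
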(event OnComponentBeginOverlap(BoxOverlap)
  (params (OverlappedComponent :type Primitive%20Component%20Object%20Reference) (OtherActor :type Actor%20Object%20Reference) (OtherComp :type Primitive%20Component%20Object%20Reference) (OtherBodyIndex :type Integer) (bFromSweep :type Boolean) (SweepResult :type Hit%20Result%20Structure%20%28by%20ref%29))
  (bind _returnvalue (Transformation|GetActorLocation))
  (bind _asbp_agdplayer_character (Utilities|Casting|CastToBP_AGDPlayerCharacter OtherActor))
  (if (< (Class|AGDStatsComponent|GetHealth (Variables|/Game/MyContent/PlayerCharacter/BP_AGDPlayerCharacter.BP_AGDPlayerCharacter_C|GetStatsComponent _asbp_agdplayer_character)) (Class|AGDStatsComponent|GetMaxHealth (Variables|/Game/MyContent/PlayerCharacter/BP_AGDPlayerCharacter.BP_AGDPlayerCharacter_C|GetStatsComponent _asbp_agdplayer_character)))
    (Class|AGDStatsComponent|SetHealth (Variables|/Game/MyContent/PlayerCharacter/BP_AGDPlayerCharacter.BP_AGDPlayerCharacter_C|GetStatsComponent _asbp_agdplayer_character) (Math|Conversions|ToFloat(Integer) (Math|Float|Ceil (Math|Float|Clamp(Float) (* (+ (Class|AGDStatsComponent|GetHealth (Variables|/Game/MyContent/PlayerCharacter/BP_AGDPlayerCharacter.BP_AGDPlayerCharacter_C|GetStatsComponent _asbp_agdplayer_character)) 5.0) 1.25) 0.0 (Class|AGDStatsComponent|GetMaxHealth (Variables|/Game/MyContent/PlayerCharacter/BP_AGDPlayerCharacter.BP_AGDPlayerCharacter_C|GetStatsComponent _asbp_agdplayer_character))))))
    (Audio|PlaySoundatLocation "/Game/MyContent/Pickups/Sound/Pickup_Stats_Cue.Pickup_Stats_Cue" _returnvalue "0, 0, 0" 1.0 1.0 0.0 0 0 0 0)
    (Effects|SpawnEmitteratLocation "/Game/InfinityBladeEffects/Effects/FX_Monsters/FX_Monster_Ausar/P_AU_Heal_01.P_AU_Heal_01" _returnvalue)
    (Actor|DestroyActor)))

(fn ConstructionScript)