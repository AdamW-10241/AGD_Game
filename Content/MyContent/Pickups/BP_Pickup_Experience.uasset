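; Experience pickup that grants the player character a fixed amount of experience on overlap, with a sound and particle burst, then destroys itself.
; Placed pickups with a PickupIndex register it in the GI_Spellblade game instance's RememberedActors and destroy themselves on BeginPlay if already collected.
; Pickups with an empty index, treated as spawned, skip that persistence step.
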(event OnComponentBeginOverlap(BoxOverlap)
  (params (OverlappedComponent :type Primitive%20Component%20Object%20Reference) (OtherActor :type Actor%20Object%20Reference) (OtherComp :type Primitive%20Component%20Object%20Reference) (OtherBodyIndex :type Integer) (bFromSweep :type Boolean) (SweepResult :type Hit%20Result%20Structure%20%28by%20ref%29))
  (bind _returnvalue (Transformation|GetActorLocation))
  (bind _asbp_agdplayer_character (Utilities|Casting|CastToBP_AGDPlayerCharacter OtherActor))
  (Class|AGDStatsComponent|AddExperience (Variables|/Game/MyContent/PlayerCharacter/BP_AGDPlayerCharacter.BP_AGDPlayerCharacter_C|GetStatsComponent _asbp_agdplayer_character) 500)
  (Audio|PlaySoundatLocation "/Game/MyContent/Pickups/Sound/Pickup_Stats_Cue.Pickup_Stats_Cue" _returnvalue "0, 0, 0" 1.0 1.0 0.0 0 0 0 0)
  (Effects|SpawnEmitteratLocation "/Game/InfinityBladeEffects/Effects/FX_Monsters/FX_Monster_Ausar/P_AU_Trap_Charge_01.P_AU_Trap_Charge_01" _returnvalue)
  (if (not (Utilities|Array|IsEmpty (Variables|Default|GetPickupIndex))) ; If has index (not spawned)
    (bind _asgi_spellblade (Utilities|Casting|CastToGI_Spellblade (Game|GetGameInstance)))
    (Utilities|Array|Add (Variables|/Game/MyContent/Core/GI_Spellblade.GI_Spellblade_C|GetRememberedActors _asgi_spellblade) (Variables|Default|GetPickupIndex)))
  (Actor|DestroyActor))

(event EventBeginPlay
  (bind _asgi_spellblade (Utilities|Casting|CastToGI_Spellblade (Game|GetGameInstance)))
  (if (Utilities|Array|ContainsItem (Variables|/Game/MyContent/Core/GI_Spellblade.GI_Spellblade_C|GetRememberedActors _asgi_spellblade) (Variables|Default|GetPickupIndex))
    (Actor|DestroyActor)))

(fn ConstructionScript)