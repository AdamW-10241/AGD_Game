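; BP_Pickup_Stamina is a pickup that restores stamina to the player character on overlap, then destroys itself.
; The box overlap adds a flat amount to current stamina, scales the sum, clamps it to the maximum, rounds it up and writes it to the character's StatsComponent.
; It plays a pickup sound and traces downward to place an ice-shatter particle at the hit location.
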(event OnComponentBeginOverlap(BoxOverlap)
  (params (OverlappedComponent :type Primitive%20Component%20Object%20Reference) (OtherActor :type Actor%20Object%20Reference) (OtherComp :type Primitive%20Component%20Object%20Reference) (OtherBodyIndex :type Integer) (bFromSweep :type Boolean) (SweepResult :type Hit%20Result%20Structure%20%28by%20ref%29))
  (bind _returnvalue (Transformation|GetActorLocation))
  (bind _asbp_agdplayer_character (Utilities|Casting|CastToBP_AGDPlayerCharacter OtherActor))
  (Class|AGDStatsComponent|SetStamina (Variables|/Game/MyContent/PlayerCharacter/BP_AGDPlayerCharacter.BP_AGDPlayerCharacter_C|GetStatsComponent _asbp_agdplayer_character) (Math|Conversions|ToFloat(Integer) (Math|Float|Ceil (Math|Float|Clamp(Float) (* (+ (Class|AGDStatsComponent|GetStamina (Variables|/Game/MyContent/PlayerCharacter/BP_AGDPlayerCharacter.BP_AGDPlayerCharacter_C|GetStatsComponent _asbp_agdplayer_character)) 5.0) 1.25) 0.0 (Class|AGDStatsComponent|GetMaxStamina (Variables|/Game/MyContent/PlayerCharacter/BP_AGDPlayerCharacter.BP_AGDPlayerCharacter_C|GetStatsComponent _asbp_agdplayer_character))))))
  (Audio|PlaySoundatLocation "/Game/MyContent/Pickups/Sound/Pickup_Stats_Cue.Pickup_Stats_Cue" _returnvalue "0, 0, 0" 1.0 1.0 0.0 0 0 0 0)
  (bind _outhit (Collision|LineTraceByChannel _returnvalue (+ _returnvalue "0.000000,0.000000,-200.000000") "TraceTypeQuery1" false 0 "None"))
  (Effects|SpawnEmitteratLocation "/Game/InfinityBladeEffects/Effects/FX_Skill_Aura/P_Aura_Ice_Shatter_01.P_Aura_Ice_Shatter_01" (.location _outhit) "0, 0, 0" "0.500000,0.500000,0.500000")
  (Actor|DestroyActor))

(fn ConstructionScript)