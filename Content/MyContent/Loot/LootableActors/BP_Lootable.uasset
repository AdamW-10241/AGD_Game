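; BP_Lootable is a world actor that players can loot once.
; Its range trigger adds or removes its loot component in the player character's Lootables and toggles a widget.
; Looting deactivates it, plays a sound and, if it has a LootableIndex (placed, not spawned), records that index in the game instance's RememberedActors.
; On BeginPlay it deactivates itself if the save game already remembers that index.
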(event OnComponentBeginOverlap(LootRange)
  (params (OverlappedComponent :type Primitive%20Component%20Object%20Reference) (OtherActor :type Actor%20Object%20Reference) (OtherComp :type Primitive%20Component%20Object%20Reference) (OtherBodyIndex :type Integer) (bFromSweep :type Boolean) (SweepResult :type Hit%20Result%20Structure%20%28by%20ref%29))
  (if (not (Variables|Default|GetbLooted))
    (bind _asbp_agdplayer_character (Utilities|Casting|CastToBP_AGDPlayerCharacter OtherActor))
    (Utilities|Array|Add (Variables|/Game/MyContent/PlayerCharacter/BP_AGDPlayerCharacter.BP_AGDPlayerCharacter_C|GetLootables _asbp_agdplayer_character) (Variables|Default|GetBP_LootComponent))
    (Rendering|SetVisibility (Variables|Default|GetWidget) true false)))

(event OnComponentEndOverlap(LootRange)
  (params (OverlappedComponent :type Primitive%20Component%20Object%20Reference) (OtherActor :type Actor%20Object%20Reference) (OtherComp :type Primitive%20Component%20Object%20Reference) (OtherBodyIndex :type Integer))
  (if (not (Variables|Default|GetbLooted))
    (bind _asbp_agdplayer_character (Utilities|Casting|CastToBP_AGDPlayerCharacter OtherActor))
    (Utilities|Array|RemoveItem (Variables|/Game/MyContent/PlayerCharacter/BP_AGDPlayerCharacter.BP_AGDPlayerCharacter_C|GetLootables _asbp_agdplayer_character) (Variables|Default|GetBP_LootComponent))
    (Rendering|SetVisibility (Variables|Default|GetWidget) false false)))

(event OnLooted(BP_LootComponent)
  (bind _audio (Variables|Default|GetAudio))
  (CallFunction|Deactivate)
  (Audio|SpawnSoundatLocation (Variables|/Script/Engine.AudioComponent|GetSound _audio) (Transformation|GetWorldLocation _audio) "0, 0, 0" 1.0 1.0 0.0 0 0)
  (if (not (Utilities|Array|IsEmpty (Variables|Default|GetLootableIndex))) ; If has index (not spawned)
    (bind _asgi_spellblade (Utilities|Casting|CastToGI_Spellblade (Game|GetGameInstance)))
    (Utilities|Array|Add (Variables|/Game/MyContent/Core/GI_Spellblade.GI_Spellblade_C|GetRememberedActors _asgi_spellblade) (Variables|Default|GetLootableIndex))))

(event Custom|Deactivate
  (Variables|Default|SetbLooted true)
  (Rendering|SetVisibility (Variables|Default|GetWidget) false false))

(event EventBeginPlay
  (bind _asgi_spellblade (Utilities|Casting|CastToGI_Spellblade (Game|GetGameInstance)))
  (Utilities|IsValid (Variables|/Game/MyContent/Core/GI_Spellblade.GI_Spellblade_C|GetSaveGameObject _asgi_spellblade)
    (:Is%20Valid
      (if (Utilities|Array|ContainsItem (Variables|/Game/MyContent/Core/BP_AGDSaveGame.BP_AGDSaveGame_C|GetRememberedActors (Variables|/Game/MyContent/Core/GI_Spellblade.GI_Spellblade_C|GetSaveGameObject _asgi_spellblade)) (Variables|Default|GetLootableIndex))
        (CallFunction|Deactivate)))))

(fn ConstructionScript)