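; BP_Checkpoint is a checkpoint actor that saves the game when the player character overlaps it.
; On BeginPlay it binds to the saving, success and failure notifications of GI_Spellblade.
; Overlap records itself as the game instance's last active checkpoint and requests a save, using a GameIsSaving flag to block repeat requests.
; Success or failure clears the flag, and success also calls OnGameSaved, currently an empty hook.
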(event Custom|OnSaving)

(event Custom|OnSuccessfulSave
  (Variables|Default|SetbGameIsSaving false)
  (CallFunction|OnGameSaved))

(event Custom|OnFailedSave
  (Variables|Default|SetbGameIsSaving false))

(event Collision|EventActorBeginOverlap
  (params (OtherActor :type Actor%20Object%20Reference))
  (if (and (== OtherActor (Game|GetPlayerCharacter 0)) (not (Variables|Default|GetbGameIsSaving)))
    (bind _agdgameinstance (Variables|Default|GetAGDGameInstance)
      (:then
        (Variables|/Game/MyContent/Core/GI_Spellblade.GI_Spellblade_C|SetLastActiveCheckpoint _agdgameinstance self)
        (Default|TrySaveGame (Variables|Default|GetAGDGameInstance))
        (Variables|Default|SetbGameIsSaving true))
      (:else))))

(event EventBeginPlay
  (bind _asgi_spellblade (Utilities|Casting|CastToGI_Spellblade (Game|GetGameInstance)))
  (Variables|Default|SetAGDGameInstance _asgi_spellblade)
  (EventDispatchers|BindEventtoSavingGame (Variables|Default|GetAGDGameInstance) (EventDispatchers|CreateEvent :!event Custom|OnSaving))
  (EventDispatchers|BindEventtoSavingGameSuccessful (Variables|Default|GetAGDGameInstance) (EventDispatchers|CreateEvent :!event Custom|OnSuccessfulSave))
  (EventDispatchers|BindEventtoSavingGameFailed (Variables|Default|GetAGDGameInstance) (EventDispatchers|CreateEvent :!event Custom|OnFailedSave)))

(fn ConstructionScript)

(fn OnGameSaved)