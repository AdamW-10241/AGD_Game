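; Enemy character Blueprint that handles hurt reactions, death, basic attacks and a health bar widget.
; StatsComponent's OnHurt turns the enemy toward the damage cause, knocks it back and updates health.
; Non-lethal hits play a reaction and interrupt BP_EnemyController; death runs once, stopping AI and movement, granting player experience, then removing the enemy after its animation.
; Animations are triggered through anim instance interface messages, with returned values timing death and attacks.
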(event OnHurt(StatsComponent)
  (params (Damage :type Float%20%28double-precision%29) (IsDead :type Boolean) (DamageCauser :type Actor%20Object%20Reference) (DamageType :type Damage%20Type%20Object%20Reference))
  (CallFunction|RotateandKnockback DamageCauser)
  (CallFunction|UpdateHealthPercent)
  (if IsDead
    (Utilities|FlowControl|DoOnce false
      (:Completed
        (CallFunction|OnDeath)
        (AI|Logic|StopLogic (Variables|/Script/AIModule.AIController|GetBrainComponent (AI|GetAIController self)) "Dead")
        (Components|Movement|StopMovementImmediately (Variables|Character|GetCharacterMovement))
        (CallFunction|GivePlayerExperience)
        (bind _duration (Class|BIEnemyAnimations|EAnimDeath(Message) (Components|SkeletalMesh|GetAnimInstance (Variables|Character|GetMesh))))
        (Utilities|FlowControl|Delay _duration)
        (Rendering|SetVisibility (Variables|Default|GetHealthBar) false false)
        (Actor|SetLifeSpan 3.0)))
    (else
      (CallFunction|TakeDamage))))

(event Custom|OnDeath)

(event EventBeginPlay
  (CallFunction|UpdateHealthPercent))

(fn ConstructionScript)

(fn RotateandKnockback
  (params (DamageCauser :type Actor%20Object%20Reference))
  (Transformation|SetActorRotation (Math|Rotator|MakeRotator 0.0 0.0 (.yaw (Math|Rotator|FindLookatRotation (Transformation|GetActorLocation) (Transformation|GetActorLocation DamageCauser)))))
  (Character|LaunchCharacter (* (Math|Vector|NegateVector (Transformation|GetActorForwardVector)) 7.5e+02) true false))

(fn UpdateHealthPercent
  (bind _statscomponent (Variables|Default|GetStatsComponent))
  (bind _aswui_enemy_health (Utilities|Casting|CastToWUI_EnemyHealth (UserInterface|GetWidget (Variables|Default|GetHealthBar))))
  (Default|SetHealthPercent _aswui_enemy_health (Class|AGDStatsComponent|GetHealth _statscomponent) (Class|AGDStatsComponent|GetMaxHealth _statscomponent)))

(fn GivePlayerExperience
  (bind _asbp_agdplayer_character (Utilities|Casting|CastToBP_AGDPlayerCharacter (Game|GetPlayerCharacter 0)))
  (Class|AGDStatsComponent|AddExperience (Variables|/Game/MyContent/PlayerCharacter/BP_AGDPlayerCharacter.BP_AGDPlayerCharacter_C|GetStatsComponent _asbp_agdplayer_character) (Variables|Experience|GetExperience)))

(fn SetAIInterupt
  (params (Bool%20Value :type Boolean))
  (bind _asbp_enemy_controller (Utilities|Casting|CastToBP_EnemyController (Pawn|GetController)))
  (Default|SetAIInterupt _asbp_enemy_controller Bool%20Value))

(fn TakeDamage
  (Class|BIEnemyAnimations|EAnimTakeDamage(Message) (Components|SkeletalMesh|GetAnimInstance (Variables|Character|GetMesh)))
  (CallFunction|SetAIInterupt true))

(fn EActionsBasicAttack
  (bind _duration (Class|BIEnemyAnimations|EAnimBasicAttack(Message) (Components|SkeletalMesh|GetAnimInstance (Variables|Character|GetMesh)) (Class|AGDStatsComponent|GetAttackSpeed (Variables|Default|GetStatsComponent))))
  (return _duration))

(fn EStatsGetAttackRange
  (return (Class|AGDEnemyCharacter|GetAttackRange)))