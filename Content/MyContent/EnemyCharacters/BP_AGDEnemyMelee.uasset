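; BP_AGDEnemyMelee is a melee enemy character that damages player characters within its hit area.
; The EActionsApplyDamage event calls MeleeDamage, which finds every BP_AGDPlayerCharacter overlapping the DamageBox.
; Each one receives damage equal to the base damage from StatsComponent, with the enemy as damage causer.
; The construction script only runs the parent's version.
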(event EventEActionsApplyDamage
  (CallFunction|MeleeDamage))

(fn ConstructionScript
  (|CallParentFunction))

(fn MeleeDamage
  (for _array_element (Collision|GetOverlappingActors (Variables|Default|GetDamageBox) "/Game/MyContent/PlayerCharacter/BP_AGDPlayerCharacter.BP_AGDPlayerCharacter_C" :!class /Script/Engine.PrimitiveComponent)
    (Game|Damage|ApplyDamage _array_element (Math|Conversions|ToFloat(Integer) (Class|AGDStatsComponent|GetBaseDamage (Variables|Default|GetStatsComponent))) 0 self)))