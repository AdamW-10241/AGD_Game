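; Dragon enemy character that fights with a fire breath effect and a leap attack, and can switch between grounded and airborne states.
; Events toggle the flamethrower particles and the leap hitbox, both switched off at BeginPlay.
; The apply-damage event deals the stats component's base damage to player characters overlapping that hitbox.
; Helpers toggle capsule collision with gravity and pass airborne state to the dragon controller, whose focus clears on death.
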(event EventAEStartParticles
  (Components|Activation|Activate (Variables|Default|GetFireEffect) true)
  (Components|Activation|Activate (Variables|Default|GetFlamethrowerEffect) true))

(event EventAEEndParticles
  (Components|Activation|Deactivate (Variables|Default|GetFireEffect))
  (Components|Activation|Deactivate (Variables|Default|GetFlamethrowerEffect)))

(event EventAEActivateHitbox
  (Collision|SetCollisionEnabled (Variables|Default|GetLeapAttackHitbox) "QueryOnly"))

(event EventAEDeactivateHitbox
  (Collision|SetCollisionEnabled (Variables|Default|GetLeapAttackHitbox) "NoCollision"))

(event EventOnCharacterDeath
  (bind _asbp_enemy_controller_dragon (Utilities|Casting|CastToBP_EnemyController_Dragon (Pawn|GetController)))
  (AI|ClearFocus _asbp_enemy_controller_dragon)
  (CallFunction|AEEndParticles))

(event EventBeginPlay
  (|CallParentFunction)
  (Variables|Default|SetbDoTakeKnockback false)
  (CallFunction|AEEndParticles)
  (Class|BIEnemyExtrasAnim|AEDeactivateHitbox(Message) self)
  (Transformation|AttachComponentToComponent (Variables|Default|GetHealthBar) (Variables|Character|GetMesh) "Root" "KeepRelative" "KeepRelative" "KeepRelative" true))

(event EventEActionsApplyDamage
  (CallFunction|LeapDamage))

(fn ConstructionScript
  (|CallParentFunction))

(fn LeapDamage
  (for _array_element (Collision|GetOverlappingActors (Variables|Default|GetLeapAttackHitbox) "/Game/MyContent/PlayerCharacter/BP_AGDPlayerCharacter.BP_AGDPlayerCharacter_C" :!class /Script/Engine.PrimitiveComponent)
    (Game|Damage|ApplyDamage _array_element (Math|Conversions|ToFloat(Integer) (Class|AGDStatsComponent|GetBaseDamage (Variables|Default|GetStatsComponent))) 0 self)))

(fn SetCollision
  (params (EnableCollision :type Boolean))
  (if EnableCollision
    (Collision|SetCollisionEnabled (Variables|Default|GetCapsuleComponent) "QueryAndPhysics")
    (Physics|SetEnableGravity (Variables|Default|GetCapsuleComponent) true)
    (else
      (Collision|SetCollisionEnabled (Variables|Default|GetCapsuleComponent) "NoCollision")
      (Physics|SetEnableGravity (Variables|Default|GetCapsuleComponent) false))))

(fn SetAirborne
  (params (bToAirborne :type Boolean))
  (if bToAirborne
    (Variables|Default|SetbIsAirborne true)
    (bind _asbp_enemy_controller_dragon (Utilities|Casting|CastToBP_EnemyController_Dragon (Pawn|GetController)))
    (Default|SetAirborne _asbp_enemy_controller_dragon true)
    (else
      (Variables|Default|SetbIsAirborne false)
      (bind _asbp_enemy_controller_dragon_2 (Utilities|Casting|CastToBP_EnemyController_Dragon (Pawn|GetController)))
      (Default|SetAirborne _asbp_enemy_controller_dragon_2 false))))

(fn PlayAnnoyedSound
  (|CallParentFunction)
  (Audio|PlaySoundatLocation "/Game/MyContent/EnemyCharacters/Sound/Dragon/dragon_growl_Cue.dragon_growl_Cue" (Transformation|GetWorldLocation (Variables|Character|GetMesh)) "0, 0, 0" 1.0 1.0 0.0 0 "/Game/MyContent/EnemyCharacters/Sound/AGD_SC.AGD_SC" 0 0))