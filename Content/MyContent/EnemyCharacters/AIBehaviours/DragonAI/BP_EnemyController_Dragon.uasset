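; AI controller for the dragon enemy that runs its behavior tree, retrying on a timer until it starts, then stores the spawn location in the Blackboard.
; Perception of the player sets or clears the target actor and adjusts the game mode's count of enemies seeing the player to update battle music.
; Death also decrements that count, and helper functions write the interrupted and airborne Blackboard flags.
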(event OnTargetPerceptionUpdated(AIPerception)
  (params (Actor :type Actor%20Object%20Reference) (Stimulus :type AI%20Stimulus%20Structure))
  (bind _output_get (Variables|Default|SetSensedActor Actor))
  (if (== _output_get (Game|GetPlayerCharacter 0))
    (if (.bSuccessfullySensed (Utilities|Struct|BreakAIStimulus Stimulus))
      (CallFunction|SetBBTargetActor (Variables|Default|GetSensedActor))
      (CallFunction|MusicAddActor)
      (else
        (CallFunction|SetBBTargetActor)
        (CallFunction|MusicRemoveActor)))))

(event Custom|CheckBehaviourTree
  (bind _returnvalue (AI|RunBehaviorTree "/Game/MyContent/EnemyCharacters/AIBehaviours/DragonAI/BT_Enemy_Dragon.BT_Enemy_Dragon"))
  (if _returnvalue
    (CallFunction|SetDefaultKeys)
    (else
      (Utilities|Time|SetTimerbyFunctionName 0 "CheckBehaviourTree" 0.5))))

(event Custom|MusicRemoveActor
  (bind _asbp_agdgm_main (Utilities|Casting|CastToBP_AGDGM_Main (Game|GetGameMode)))
  (bind _asbp_agdenemy_character (Utilities|Casting|CastToBP_AGDEnemyCharacter (Pawn|GetControlledPawn)))
  (Math|Integer|DecrementInt (Variables|/Game/MyContent/Core/BP_AGDGM_Main.BP_AGDGM_Main_C|GetEnemiesThatSeePlayer _asbp_agdgm_main)
    (:%20%20
      (Default|UpdateMusic _asbp_agdgm_main (Variables|/Game/MyContent/EnemyCharacters/BP_AGDEnemyCharacter.BP_AGDEnemyCharacter_C|GetBattleMusic _asbp_agdenemy_character)))))

(event Custom|MusicAddActor
  (bind _asbp_agdgm_main (Utilities|Casting|CastToBP_AGDGM_Main (Game|GetGameMode)))
  (bind _asbp_agdenemy_character (Utilities|Casting|CastToBP_AGDEnemyCharacter (Pawn|GetControlledPawn)))
  (Math|Integer|IncrementInt (Variables|/Game/MyContent/Core/BP_AGDGM_Main.BP_AGDGM_Main_C|GetEnemiesThatSeePlayer _asbp_agdgm_main)
    (:%20%20
      (Default|UpdateMusic _asbp_agdgm_main (Variables|/Game/MyContent/EnemyCharacters/BP_AGDEnemyCharacter.BP_AGDEnemyCharacter_C|GetBattleMusic _asbp_agdenemy_character)))))

(event EventBeginPlay
  (bind _returnvalue (AI|RunBehaviorTree "/Game/MyContent/EnemyCharacters/AIBehaviours/DragonAI/BT_Enemy_Dragon.BT_Enemy_Dragon"))
  (if _returnvalue
    (CallFunction|SetDefaultKeys)
    (else
      (Utilities|Time|SetTimerbyFunctionName 0 "CheckBehaviourTree" 0.5))))

(event EventOnDeath
  (CallFunction|MusicRemoveActor))

(fn ConstructionScript)

(fn SetDefaultKeys
  (AI|Components|Blackboard|SetValueasVector (AI|GetBlackboard 0) (Utilities|Name|MakeLiteralName "StartLocation") (Transformation|GetActorLocation (Pawn|GetControlledPawn))))

(fn SetBBTargetActor
  (params (Actor :type Object%20Object%20Reference))
  (AI|Components|Blackboard|SetValueasObject (AI|GetBlackboard 0) (Utilities|Name|MakeLiteralName "TargetActor") Actor))

(fn SetAIInterrupt
  (params (BoolValue :type Boolean))
  (AI|Components|Blackboard|SetValueasBool (AI|GetBlackboard 0) (Utilities|Name|MakeLiteralName "bIsInterrupted") BoolValue))

(fn SetAirborne
  (params (Bool%20Value :type Boolean))
  (AI|Components|Blackboard|SetValueasBool (AI|GetBlackboard 0) (Utilities|Name|MakeLiteralName "bIsAirborne") Bool%20Value))