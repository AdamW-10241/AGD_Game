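; Default enemy AI controller that runs BT_Enemy_Default on possess, retrying on a timer until it starts, then stores the start location.
; Perception sets or clears the player as blackboard target.
; The same sight changes adjust the game mode's count of enemies seeing the player and update battle music, guarded against double counting and released on death.
; Tick flags the enemy mature after a set time alive, and a helper sets an interrupt key.
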(event OnTargetPerceptionUpdated(AIPerception)
  (params (Actor :type Actor%20Object%20Reference) (Stimulus :type AI%20Stimulus%20Structure))
  (bind _output_get (Variables|Default|SetSensedActor Actor))
  (if (== _output_get (Game|GetPlayerCharacter 0))
    (if (.bSuccessfullySensed (Utilities|Struct|BreakAIStimulus Stimulus))
      (CallFunction|SetBBTargetActor (Variables|Default|GetSensedActor))
      (CallFunction|MusicAddActor)
      (else
        (CallFunction|SetBBTargetActor)
        (CallFunction|MusicRemoveActor)))))

(event Custom|CheckBehaviourTree
  (bind _returnvalue (AI|RunBehaviorTree "/Game/MyContent/EnemyCharacters/AIBehaviours/DefaultAI/BT_Enemy_Default.BT_Enemy_Default"))
  (if _returnvalue
    (CallFunction|SetDefaultKeys)
    (else
      (Utilities|Time|SetTimerbyFunctionName 0 "CheckBehaviourTree" 0.5))))

(event Custom|MusicAddActor
  (if (not (Variables|Default|GetbIsAdded))
    (bind _asbp_agdgm_main (Utilities|Casting|CastToBP_AGDGM_Main (Game|GetGameMode)))
    (bind _asbp_agdenemy_character (Utilities|Casting|CastToBP_AGDEnemyCharacter (Pawn|GetControlledPawn)))
    (Math|Integer|IncrementInt (Variables|/Game/MyContent/Core/BP_AGDGM_Main.BP_AGDGM_Main_C|GetEnemiesThatSeePlayer _asbp_agdgm_main)
      (:%20%20
        (Default|UpdateMusic _asbp_agdgm_main (Variables|/Game/MyContent/EnemyCharacters/BP_AGDEnemyCharacter.BP_AGDEnemyCharacter_C|GetBattleMusic _asbp_agdenemy_character) false false)
        (Variables|Default|SetbIsAdded true)))))

(event Custom|MusicRemoveActor
  (if (Variables|Default|GetbIsAdded)
    (bind _asbp_agdgm_main (Utilities|Casting|CastToBP_AGDGM_Main (Game|GetGameMode)))
    (bind _asbp_agdenemy_character (Utilities|Casting|CastToBP_AGDEnemyCharacter (Pawn|GetControlledPawn)))
    (Math|Integer|DecrementInt (Variables|/Game/MyContent/Core/BP_AGDGM_Main.BP_AGDGM_Main_C|GetEnemiesThatSeePlayer _asbp_agdgm_main)
      (:%20%20
        (Default|UpdateMusic _asbp_agdgm_main (Variables|/Game/MyContent/EnemyCharacters/BP_AGDEnemyCharacter.BP_AGDEnemyCharacter_C|GetBattleMusic _asbp_agdenemy_character) false false)
        (Variables|Default|SetbIsAdded false)))))

(event EventTick
  (params (DeltaSeconds :type Float%20%28single-precision%29))
  (if (not (Variables|Default|GetbIsMature))
    (bind _output_get (Variables|Default|SetTimeAlive (+ DeltaSeconds (Variables|Default|GetTimeAlive))))
    (if (>= _output_get (Variables|Default|GetTimeToMature))
      (CallFunction|SetMature true))))

(event EventPossess
  (params (PossessedPawn :type Pawn%20Object%20Reference))
  (bind _returnvalue (AI|RunBehaviorTree "/Game/MyContent/EnemyCharacters/AIBehaviours/DefaultAI/BT_Enemy_Default.BT_Enemy_Default"))
  (if _returnvalue
    (CallFunction|SetDefaultKeys)
    (else
      (Utilities|Time|SetTimerbyFunctionName 0 "CheckBehaviourTree" 0.5))))

(event EventOnDeath
  (CallFunction|MusicRemoveActor))

(fn ConstructionScript)

(fn SetDefaultKeys
  (AI|Components|Blackboard|SetValueasVector (AI|GetBlackboard 0) (Utilities|Name|MakeLiteralName "StartLocation") (Transformation|GetActorLocation (Pawn|GetControlledPawn))))

(fn SetBBTargetActor
  (params (Actor :type Object%20Object%20Reference))
  (AI|Components|Blackboard|SetValueasObject (AI|GetBlackboard 0) (Utilities|Name|MakeLiteralName "TargetActor") Actor))

(fn SetAIInterrupt
  (params (BoolValue :type Boolean))
  (AI|Components|Blackboard|SetValueasBool (AI|GetBlackboard 0) (Utilities|Name|MakeLiteralName "bIsInterrupted") BoolValue))

(fn SetMature
  (params (BoolValue :type Boolean))
  (bind _output_get (Variables|Default|SetbIsMature BoolValue))
  (AI|Components|Blackboard|SetValueasBool (AI|GetBlackboard 0) (Utilities|Name|MakeLiteralName "bIsMature") _output_get))