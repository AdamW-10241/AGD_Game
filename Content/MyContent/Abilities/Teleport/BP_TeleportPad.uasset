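; BP_TeleportPad is a teleport pad that moves the player to its TeleportPoint when the player triggers a teleport while standing in range.
; On BeginPlay it binds to the player character's PlayerTeleport event.
; Overlapping TeleportRange sets CanTeleport on the character, tracks PlayerInRange and toggles a widget.
; On the event, the in-range pad teleports the player pawn and activates its particle and audio components.
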(event OnComponentBeginOverlap(TeleportRange)
  (params (OverlappedComponent :type Primitive%20Component%20Object%20Reference) (OtherActor :type Actor%20Object%20Reference) (OtherComp :type Primitive%20Component%20Object%20Reference) (OtherBodyIndex :type Integer) (bFromSweep :type Boolean) (SweepResult :type Hit%20Result%20Structure%20%28by%20ref%29))
  (bind _asbp_agdplayer_character (Utilities|Casting|CastToBP_AGDPlayerCharacter OtherActor))
  (Variables|/Game/MyContent/PlayerCharacter/BP_AGDPlayerCharacter.BP_AGDPlayerCharacter_C|SetbCanTeleport _asbp_agdplayer_character true)
  (Variables|Default|SetbPlayerInRange true)
  (Rendering|SetVisibility (Variables|Default|GetWidget) true false))

(event OnComponentEndOverlap(TeleportRange)
  (params (OverlappedComponent :type Primitive%20Component%20Object%20Reference) (OtherActor :type Actor%20Object%20Reference) (OtherComp :type Primitive%20Component%20Object%20Reference) (OtherBodyIndex :type Integer))
  (bind _asbp_agdplayer_character (Utilities|Casting|CastToBP_AGDPlayerCharacter OtherActor))
  (Variables|/Game/MyContent/PlayerCharacter/BP_AGDPlayerCharacter.BP_AGDPlayerCharacter_C|SetbCanTeleport _asbp_agdplayer_character false)
  (Variables|Default|SetbPlayerInRange false)
  (Rendering|SetVisibility (Variables|Default|GetWidget) false false))

(event Custom|TeleportPlayer
  (if (Variables|Default|GetbPlayerInRange)
    (Transformation|SetActorTransform (Game|Player|GetPlayerPawn 0) (Transformation|GetWorldTransform (Variables|Default|GetTeleportPoint)) false true)
    (Components|Activation|Activate (Variables|Default|GetParticleSystem) false)
    (Components|Activation|Activate (Variables|Default|GetAudio) false)))

(event EventBeginPlay
  (bind _asbp_agdplayer_character (Utilities|Casting|CastToBP_AGDPlayerCharacter (Game|Player|GetPlayerPawn 0)))
  (EventDispatchers|BindEventtoPlayerTeleport _asbp_agdplayer_character (delegate Custom|TeleportPlayer)))

(fn ConstructionScript)