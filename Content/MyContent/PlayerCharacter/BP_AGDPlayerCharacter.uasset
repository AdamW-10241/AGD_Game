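; BP_AGDPlayerCharacter is the player's melee character, with combo attacks, a cooldown-gated AOE special that spawns a rock-fire burst, and level-up effects.
; A toggleable hitbox applies StatsComponent's base damage to overlapped actors, and animation work goes through messages to the AnimInstance.
; Stat events refresh health and stamina widgets, while hurt triggers an interruptible reaction and death reloads the level.
; Tick enables controller-facing rotation while moving outside attacks and montages, or when forced.
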(event LevelledUp(StatsComponent)
  (params (Level :type Integer) (bAreStatsInitialised :type Boolean))
  ;[1 1 1] Level up
  (if bAreStatsInitialised ; Only run if not initialising
    (Effects|SpawnEmitteratLocation "/Game/InfinityBladeEffects/Effects/FX_Mobile/Misc/P_levelUp.P_levelUp" (Transformation|GetActorLocation))
    (CallFunction|UpdateWidget)))

(event OnComponentBeginOverlap(DamageHitbox)
  (params (OverlappedComponent :type Primitive%20Component%20Object%20Reference) (OtherActor :type Actor%20Object%20Reference) (OtherComp :type Primitive%20Component%20Object%20Reference) (OtherBodyIndex :type Integer) (bFromSweep :type Boolean) (SweepResult :type Hit%20Result%20Structure%20%28by%20ref%29))
  ;[1 1 1] Apply Damage to Everything
  (if (!= OtherActor self)
    (Game|Damage|ApplyDamage OtherActor (Math|Conversions|ToFloat(Integer) (Class|AGDStatsComponent|GetBaseDamage (Variables|Default|GetStatsComponent))) 0 self)))

(event OnHurt(StatsComponent)
  (params (Damage :type Float%20%28double-precision%29) (IsDead :type Boolean) (DamageCauser :type Actor%20Object%20Reference) (DamageType :type Damage%20Type%20Object%20Reference))
  (bind _returnvalue (Game|GetPlayerController 0))
  ;[1 1 1] On Hurt / Death
  (CallFunction|UpdateWidget)
  (if IsDead
    (Input|DisableInput _returnvalue _returnvalue)
    (bind _duration (Class|BIPlayerAnimations|PAnimDeath(Message) (Components|SkeletalMesh|GetAnimInstance (Variables|Character|GetMesh))))
    (Utilities|FlowControl|Delay (+ _duration 2.0))
    (bind _returnvalue_2 (Game|GetCurrentLevelName true))
    (Game|OpenLevel(byName) (Utilities|String|StringToName _returnvalue_2))
    (elif (and (not (Variables|Default|GetbRecentlyTakenDamage)) (Variables|Default|GetbCanBeInterupted))
      (Variables|Default|SetbRecentlyTakenDamage true)
      (Class|AGDCharacter|FaceOtherActor DamageCauser)
      (Audio|PlaySoundatLocation "/Game/MyContent/PlayerCharacter/Sound/hurt_sound_cue.hurt_sound_cue" (Transformation|GetActorLocation) "0, 0, 0" 1.0 1.0 0.0 0 0 0 0)
      (bind _duration_2 (Class|BIPlayerAnimations|PAnimTakeDamage(Message) (Components|SkeletalMesh|GetAnimInstance (Variables|Character|GetMesh))))
      (Utilities|FlowControl|Delay (+ _duration_2 -0.5))
      (Variables|Default|SetbRecentlyTakenDamage false))))

(event EventBeginPlay
  ;[1 1 1] Begin - Update Widget
  (CallFunction|UpdateHealthWidget))

(event EventTick
  (params (DeltaSeconds :type Float%20%28single-precision%29))
  ;[1 1 1] Rotation
  (CallFunction|HandleRotation))

(fn ConstructionScript)

(fn HandleRotation
  (Variables|/Script/Engine.CharacterMovementComponent|SetbUseControllerDesiredRotation (Variables|Character|GetCharacterMovement) (or (Math|Boolean|ANDBoolean (> (Math|Vector|VectorLength (Transformation|GetVelocity)) 0.0) (Class|AGDPlayerCharacter|GetAttackAllowed) (not (CallFunction|IsAnimationMontagePlaying))) (Class|AGDPlayerCharacter|GetForceRotate))))

(fn PrimaryAttack
  (if (not (Variables|Default|GetbRecentlyTakenDamage))
    (Class|BIPlayerAnimations|PAnimPlayComboAttack(Message) (Components|SkeletalMesh|GetAnimInstance (Variables|Character|GetMesh)) (Class|AGDStatsComponent|GetAttackSpeed (Variables|Default|GetStatsComponent)))))

(fn IsAnimationMontagePlaying
  (return (Class|AnimInstance|IsAnyMontagePlaying (Components|SkeletalMesh|GetAnimInstance (Variables|Character|GetMesh)))))

(fn ActivateDamage
  (Collision|SetCollisionEnabled (Variables|Default|GetDamageHitbox) "QueryOnly"))

(fn DeactivateDamage
  (Collision|SetCollisionEnabled (Variables|Default|GetDamageHitbox) "NoCollision"))

(fn SpecialAttack
  (if (<= (Variables|Default|GetSpecialAttackCD) 0.0)
    (Variables|Default|SetbCanBeInterupted false)
    (bind _success (Class|BIPlayerAnimations|PAnimAOEAttack(Message) (Components|SkeletalMesh|GetAnimInstance (Variables|Character|GetMesh))))
    (if _success ; If successful AOE attack
      (bind _output_get (Variables|Default|SetSpecialAttackCD (Variables|Default|GetSpecialAttackCDDuration)))
      (Utilities|Time|SetTimerbyFunctionName 0 "ResetSpecialAttack" _output_get))))

(fn ResetSpecialAttack
  (Variables|Default|SetSpecialAttackCD 0.0)
  (Variables|Default|SetbCanBeInterupted true))

(fn SpawnAOEAttack
  (Game|SpawnActorfromClass "/Game/MyContent/PlayerCharacter/Abilities/Ability_RockFireBurst.Ability_RockFireBurst_C" (Math|Transform|MakeTransform (Transformation|GetWorldLocation (Variables|Default|GetFeet)) "0, 0, 0" "1.000000,1.000000,1.000000") "Undefined" "MultiplyWithRoot" self (Math|Conversions|ToFloat(Integer) (* (+ (Class|AGDStatsComponent|GetBaseDamage (Variables|Default|GetStatsComponent)) 3) 2)) 0))

(fn UpdateHealthWidget
  (bind _asbp_agdplayer_controller (Utilities|Casting|CastToBP_AGDPlayerController (Pawn|GetController)))
  (Default|UpdateHealthWidget _asbp_agdplayer_controller)
  (Default|UpdateStaminaWidget _asbp_agdplayer_controller))

(fn UpdateWidget
  (CallFunction|UpdateHealthWidget))