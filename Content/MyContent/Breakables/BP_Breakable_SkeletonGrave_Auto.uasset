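; Breakable skeleton grave that breaks automatically when the player pawn enters its overlap box.
; On first overlap it swaps to a gravestone mesh, disables that mesh's collision and snaps it to the FixedBrokenLocation component's relative position.
; It then calls Trigger and sets the Triggered flag so it fires only once.
; The Destroy event is deliberately empty, and construction defers to the parent class.
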(event OnComponentBeginOverlap(BoxOverlap)
  (params (OverlappedComponent :type Primitive%20Component%20Object%20Reference) (OtherActor :type Actor%20Object%20Reference) (OtherComp :type Primitive%20Component%20Object%20Reference) (OtherBodyIndex :type Integer) (bFromSweep :type Boolean) (SweepResult :type Hit%20Result%20Structure%20%28by%20ref%29))
  (bind _staticmesh (Variables|Default|GetStaticMesh))
  (if (not (Variables|Default|GetbTriggered))
    (if (== OtherActor (Game|Player|GetPlayerPawn 0))
      (Components|StaticMesh|SetStaticMesh _staticmesh "/Game/Grave/Gravestones_set_Gravestone_04.Gravestones_set_Gravestone_04")
      (Collision|SetCollisionEnabled _staticmesh "NoCollision")
      (Transformation|SetRelativeLocation _staticmesh (Variables|/Script/Engine.SceneComponent|GetRelativeLocation (Variables|Default|GetFixedBrokenLocation)) false false)
      (CallFunction|Trigger)
      (Variables|Default|SetbTriggered true))))

(event EventDestroy)

(fn ConstructionScript
  (|CallParentFunction))