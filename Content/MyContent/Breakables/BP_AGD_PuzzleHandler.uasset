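; BP_AGD_PuzzleHandler is a puzzle gate that opens once it has received enough trigger responses.
; Each TriggerHandler call increments a response counter, and reaching the maximum runs FinishPuzzle once.
; FinishPuzzle hides the wind wall, disables the box collision, and plays audio and particle effects.
; The effects are skipped within the first second after creation, so completions restored from a level save stay silent.
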(event Custom|TriggerHandler
  (bind _result (Math|Integer|IncrementInt (Variables|Default|GetPuzzleResponses))
    (:%20%20
      (if (>= _result (Variables|Default|GetMaxNumberOfResponses))
        (Utilities|FlowControl|DoOnce false
          (:Completed
            (CallFunction|FinishPuzzle)))))))

(event Custom|FinishPuzzle
  (Rendering|SetVisibility (Variables|Default|GetN_WindWall) false true)
  (Collision|SetCollisionEnabled (Variables|Default|GetBox) "NoCollision")
  (if (> (Actor|GetGameTimeSinceCreation) 1.0) ; If happened in first second, happened from level save and should be silent
    (Components|Activation|Activate (Variables|Default|GetAudio) false)
    (Components|Activation|Activate (Variables|Default|GetParticleSystem) false)))

(fn ConstructionScript)