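; Spider egg cluster that breaks open automatically when the player walks into its trigger volume.
; A Box overlap checks for player pawn 0 and fires only once, guarded by a Triggered flag.
; OpenBreakables loops over all child actors, including descendants, casts each to BP_Breakable_SpiderEgg and calls its Trigger.
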(event OnComponentBeginOverlap(Box)
  (params (OverlappedComponent :type Primitive%20Component%20Object%20Reference) (OtherActor :type Actor%20Object%20Reference) (OtherComp :type Primitive%20Component%20Object%20Reference) (OtherBodyIndex :type Integer) (bFromSweep :type Boolean) (SweepResult :type Hit%20Result%20Structure%20%28by%20ref%29))
  (if (not (Variables|Default|GetbTriggered))
    (if (== OtherActor (Game|Player|GetPlayerPawn 0))
      (CallFunction|OpenBreakables)
      (Variables|Default|SetbTriggered true))))

(fn ConstructionScript)

(fn OpenBreakables
  (for _array_element (Actor|GetAllChildActors true)
    (bind _asbp_breakable_spider_egg (Utilities|Casting|CastToBP_Breakable_SpiderEgg _array_element))
    (Default|Trigger _asbp_breakable_spider_egg)))