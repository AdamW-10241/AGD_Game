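; BP_AGD_Breakable is a breakable actor that shatters when the player's damage hitbox or an AGDAbility overlaps its box while active.
; Trigger runs the break sequence: play effects, spawn an optional ToSpawn class at SpawnLocation, deactivate, then destroy the actor.
; Effects spawn at location from the ParticleSystem and Audio components' assigned assets, with a sound concurrency setting applied.
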(event OnComponentBeginOverlap(BoxOverlap)
  (params (OverlappedComponent :type Primitive%20Component%20Object%20Reference) (OtherActor :type Actor%20Object%20Reference) (OtherComp :type Primitive%20Component%20Object%20Reference) (OtherBodyIndex :type Integer) (bFromSweep :type Boolean) (SweepResult :type Hit%20Result%20Structure%20%28by%20ref%29))
  (if (Variables|Default|GetbIsActive)
    (CallFunction|CheckPlayer OtherActor OtherComp)
    (CallFunction|CheckAbility OtherActor)))

(event Custom|Break
  (CallFunction|PlayFX))

(event Custom|Destroy
  (Actor|DestroyActor))

(event Custom|SpawnActor
  (CallFunction|Spawn))

(event Custom|Deactivate
  (Variables|Default|SetbIsActive false))

(event Custom|Trigger
  (CallFunction|Break)
  (CallFunction|Spawn)
  (CallFunction|Deactivate)
  (CallFunction|Destroy))

(fn ConstructionScript)

(fn PlayFX
  (bind _audio (Variables|Default|GetAudio))
  (bind _particlesystem (Variables|Default|GetParticleSystem))
  (bind _returnvalue (Transformation|GetWorldTransform _particlesystem))
  (Effects|SpawnEmitteratLocation (Variables|/Script/Engine.ParticleSystemComponent|GetTemplate _particlesystem) (.location _returnvalue) (.rotation _returnvalue) (.scale _returnvalue))
  (Audio|SpawnSoundatLocation (Variables|/Script/Engine.AudioComponent|GetSound _audio) (Transformation|GetWorldLocation _audio) "0, 0, 0" 1.0 1.0 0.0 0 "/Game/MyContent/Breakables/Sound/AGD_Breakable_SC.AGD_Breakable_SC"))

(fn Spawn
  (if (Utilities|IsValidClass (Variables|Default|GetToSpawn))
    (Game|SpawnActorfromClass (Variables|Default|GetToSpawn) (Math|Transform|MakeTransform (Transformation|GetWorldLocation (Variables|Default|GetSpawnLocation)) "0, 0, 0" "1.000000,1.000000,1.000000") "Undefined" "MultiplyWithRoot" self 0)))

(fn CheckPlayer
  (params (Object :type Object%20Object%20Reference) (Other%20Comp :type Object%20Object%20Reference))
  (bind _asbp_agdplayer_character (Utilities|Casting|CastToBP_AGDPlayerCharacter Object))
  (if (== (Variables|/Game/MyContent/PlayerCharacter/BP_AGDPlayerCharacter.BP_AGDPlayerCharacter_C|GetDamageHitbox _asbp_agdplayer_character) Other%20Comp)
    (CallFunction|Trigger)))

(fn CheckAbility
  (params (Object :type Object%20Object%20Reference))
  (Utilities|Casting|CastToAGDAbility Object)
  (CallFunction|Trigger))