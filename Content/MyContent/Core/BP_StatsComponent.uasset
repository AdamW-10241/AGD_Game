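; Stats component that handles damage and death for its owning actor and relays level-up events.
; On BeginPlay it binds to the owner's OnTakeAnyDamage and ignores further damage once dead.
; HandleDamage subtracts damage from health, clamps it between zero and max, updates IsDead and broadcasts OnHurt with the damage details.
; OnLevelUp rebroadcasts the level and stats-initialised flag through the LevelledUp dispatcher.
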(event Custom|OnOwnerTakeAnyDamage
  (params (DamagedActor :type Actor%20Object%20Reference) (Damage :type Float%20%28single-precision%29) (DamageType :type Damage%20Type%20Object%20Reference) (InstigatedBy :type Controller%20Object%20Reference) (DamageCauser :type Actor%20Object%20Reference))
  (if (not (CallFunction|IsDead))
    (CallFunction|HandleDamage Damage DamageCauser DamageType)))

(event EventOnLevelUp
  (params (Level :type Integer) (bAreStatsInitialised :type Boolean))
  (Default|CallLevelledUp Level bAreStatsInitialised))

(event EventBeginPlay
  (EventDispatchers|BindEventtoOnTakeAnyDamage (Components|GetOwner) (delegate Custom|OnOwnerTakeAnyDamage)))

(fn HandleDamage
  (params (Damage :type Float%20%28double-precision%29) (DamageCauser :type Actor%20Object%20Reference) (DamageType :type Damage%20Type%20Object%20Reference))
  (LocalVariables|SetLDamage Damage)
  (LocalVariables|SetLDamageCauser DamageCauser)
  (LocalVariables|SetLDamageType DamageType)
  (Class|AGDStatsComponent|SetHealth (Math|Float|Clamp(Float) (- (Class|AGDStatsComponent|GetHealth) Damage) 0.0 (Class|AGDStatsComponent|GetMaxHealth)))
  (bind _output_get (Variables|Default|SetbIsDead (<= (Class|AGDStatsComponent|GetHealth) 0.0)))
  (Default|CallOnHurt (LocalVariables|GetLDamage) _output_get (LocalVariables|GetLDamageCauser) (LocalVariables|GetLDamageType)))

(fn IsDead
  (return (Variables|Default|GetbIsDead)))