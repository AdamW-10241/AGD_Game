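; Menu game mode that plays background music and chooses the default pawn class by level.
; Its construction script assigns the menu player character in MainMenuLevel and the standard player character elsewhere.
; BeginPlay and the music component's finished event call UpdateMusic, which fades out, waits briefly, sets the cue and fades in.
; UpdateMusic ignores its state and boss-defeat inputs, always selecting the same legacy track.
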(event OnAudioFinished(Music)
  (CallFunction|UpdateMusic "NewEnumerator0" false))

(event Custom|UpdateMusic
  (params (MusicState :type E_AGD_MusicState%20Enum :default "NewEnumerator0") (bWasBossJustDefeated :type Boolean))
  (Variables|Default|SetNextTrack "/Game/RPG_Orchestral_Essentials_Free_Sample/Cues/LEGACY_Encounter_of_Misdeeds_WAV_Cue.LEGACY_Encounter_of_Misdeeds_WAV_Cue")
  (Audio|Components|Audio|FadeOut (Variables|Default|GetMusic) (Variables|Default|GetFadeTime) 0.0 "Linear" :!class /Script/Engine.AudioComponent)
  (Utilities|FlowControl|Delay 0.5)
  (Audio|Components|Audio|SetSound (Variables|Default|GetMusic) (Variables|Default|GetNextTrack))
  (Audio|Components|Audio|FadeIn (Variables|Default|GetMusic) (Variables|Default|GetFadeTime) 1.0 0.0 "Linear" :!class /Script/Engine.AudioComponent))

(event EventBeginPlay
  (CallFunction|UpdateMusic "NewEnumerator5" false))

(fn ConstructionScript
  (bind _returnvalue (Game|GetCurrentLevelName true))
  (if (Utilities|Enum|Equal(Enum) _returnvalue "MainMenuLevel")
    (Variables|Default|SetDefaultPawnClass "/Game/MyContent/PlayerCharacter/Menu/BP_AGDPlayerCharacter_Menu.BP_AGDPlayerCharacter_Menu_C") ; Menu
    (else
      (Variables|Default|SetDefaultPawnClass "/Game/MyContent/PlayerCharacter/BP_AGDPlayerCharacter.BP_AGDPlayerCharacter_C") ; Default
    )))