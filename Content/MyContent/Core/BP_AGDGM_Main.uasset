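; Main game mode that runs adaptive background music and assigns index strings to level actors.
; UpdateMusic picks a level or boss-defeated track when no enemy sees the player, otherwise compares state enum values to gate changes.
; Track swaps fade out, delay briefly and fade in; a finished track re-triggers the update.
; The construction script stamps enemies, breakables, pickups and lootables with IDs built from level name, type and array index.
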(event OnAudioFinished(Music)
  (CallFunction|UpdateMusic "NewEnumerator0" false))

(event Custom|UpdateMusic
  (params (MusicState :type E_AGD_MusicState%20Enum :default "NewEnumerator0") (bWasBossJustDefeated :type Boolean))
  (if (== (Variables|Default|GetEnemiesThatSeePlayer) 0)
    (if bWasBossJustDefeated
      (Variables|Default|SetMusicState "NewEnumerator4")
      (else
        (bind _returnvalue (Game|GetCurrentLevelName true))
        (switch string _returnvalue
          (:TutorialLevel
            (Variables|Default|SetMusicState "NewEnumerator0" :!label _label))
          (:Level1
            (goto _label))
          (:Level2
            (Variables|Default|SetMusicState "NewEnumerator6")))))
    (switch Utilities|FlowControl|Switch|SwitchonE_AGD_MusicState (stale _output_get) :!label _label_2
      (:NewEnumerator0
        (Variables|Default|SetNextTrack "/Game/RPG_Orchestral_Essentials_Free_Sample/Cues/LEGACY_In_Tranquil_Spring_WAV_Cue.LEGACY_In_Tranquil_Spring_WAV_Cue"))
      (:NewEnumerator1
        (Variables|Default|SetNextTrack "/Game/RPG_Orchestral_Essentials_Free_Sample/Cues/LEGACY_A_Fight_in_the_Fields_WAV_Cue.LEGACY_A_Fight_in_the_Fields_WAV_Cue"))
      (:NewEnumerator2
        (Variables|Default|SetNextTrack "/Game/RPG_Orchestral_Essentials_Free_Sample/Cues/LEGACY_Heated_Lands_WAV_Cue.LEGACY_Heated_Lands_WAV_Cue"))
      (:NewEnumerator3
        (Variables|Default|SetNextTrack "/Game/RPG_Orchestral_Essentials_Free_Sample/Cues/LEGACY_A_Slave_To_No_One_WAV_Cue.LEGACY_A_Slave_To_No_One_WAV_Cue"))
      (:NewEnumerator4
        (Variables|Default|SetNextTrack "/Game/RPG_Orchestral_Essentials_Free_Sample/Cues/LEGACY_Can_t_Stop_Winning_WAV_Cue.LEGACY_Can_t_Stop_Winning_WAV_Cue"))
      (:NewEnumerator6
        (Variables|Default|SetNextTrack "/Game/RPG_Orchestral_Essentials_Free_Sample/Cues/LEGACY_Heated_Lands_WAV_Cue.LEGACY_Heated_Lands_WAV_Cue")))
    (Audio|Components|Audio|FadeOut (Variables|Default|GetMusic) (Variables|Default|GetFadeTime) 0.0 "Linear" :!class /Script/Engine.AudioComponent)
    (Utilities|FlowControl|Delay 0.5)
    (Audio|Components|Audio|SetSound (Variables|Default|GetMusic) (Variables|Default|GetNextTrack))
    (Audio|Components|Audio|FadeIn (Variables|Default|GetMusic) (Variables|Default|GetFadeTime) 1.0 0.0 "Linear" :!class /Script/Engine.AudioComponent)
    (elif (> (Math|Conversions|ToInteger(Byte) MusicState) (Math|Conversions|ToInteger(Byte) (Variables|Default|GetMusicState)))
      (bind _output_get (Variables|Default|SetMusicState MusicState))
      (goto _label_2))))

(event EventBeginPlay
  (CallFunction|UpdateMusic "NewEnumerator5" false))

(fn ConstructionScript
  (bind _returnvalue (Game|GetCurrentLevelName true))
  (LocalVariables|SetLCurrentLevelName _returnvalue)
  (bind _outactors (Actor|GetAllActorsOfClass "/Game/MyContent/EnemyCharacters/BP_AGDEnemyCharacter.BP_AGDEnemyCharacter_C"))
  (for (_array_element _array_index) _outactors
    (Variables|/Game/MyContent/EnemyCharacters/BP_AGDEnemyCharacter.BP_AGDEnemyCharacter_C|SetEnemyIndex _array_element (Utilities|String|Append (LocalVariables|GetLCurrentLevelName) "-Enemy-" (Utilities|String|ToString(Integer) _array_index))))
  (bind _outactors_2 (Actor|GetAllActorsOfClass "/Game/MyContent/Breakables/BP_AGD_Breakable.BP_AGD_Breakable_C"))
  (for (_array_element_2 _array_index_2) _outactors_2
    (Variables|/Game/MyContent/Breakables/BP_AGD_Breakable.BP_AGD_Breakable_C|SetBreakableIndex _array_element_2 (Utilities|String|Append (LocalVariables|GetLCurrentLevelName) "-Breakable-" (Utilities|String|ToString(Integer) _array_index_2))))
  (bind _outactors_3 (Actor|GetAllActorsOfClass "/Script/AGD_Game.BP_Pickup"))
  (for (_array_element_3 _array_index_3) _outactors_3
    (Variables|/Script/AGD_Game.BP_Pickup|SetPickupIndex _array_element_3 (Utilities|String|Append (LocalVariables|GetLCurrentLevelName) "-Pickup-" (Utilities|String|ToString(Integer) _array_index_3))))
  (bind _outactors_4 (Actor|GetAllActorsOfClass "/Game/MyContent/Loot/LootableActors/BP_Lootable.BP_Lootable_C"))
  (for (_array_element_4 _array_index_4) _outactors_4
    (Variables|/Game/MyContent/Loot/LootableActors/BP_Lootable.BP_Lootable_C|SetLootableIndex _array_element_4 (Utilities|String|Append (LocalVariables|GetLCurrentLevelName) "-Lootable-" (Utilities|String|ToString(Integer) _array_index_4)))))